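; BP_Canvas is a paintable canvas for a VR painting game that can export its image as a JPG.
; On BeginPlay it creates a white render target and feeds it to the canvas mesh's dynamic material.
; OnPaintVisualTraceLine passes the hit UV and the brush's size, color and strength into a brush material, then draws that material onto the render target.
; ExportImage writes the target to a hardcoded disk path, printing on success.
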(event EventBeginPlay
  (bind _returnvalue (Rendering|Material|CreateDynamicMaterialInstance (Variables|Default|GetSM_CanvasPlat) 0 "/Game/PaintVR/Materials/MI_Canvas.MI_Canvas" "None" :!class /Script/Engine.PrimitiveComponent))
  (Variables|Default|SetDynamicInstanceMaterial _returnvalue)
  (bind _returnvalue_2 (Rendering|CreateRenderTarget2D (Variables|RenderTextire|GetRenderTextureSizeX) (Variables|RenderTextire|GetRenderTextureSizeY) "RTF_RGBA8_SRGB" "(R=1.000000,G=1.000000,B=1.000000,A=1.000000)"))
  (Variables|RenderTextire|SetRender_to_Texture _returnvalue_2)
  (Rendering|Material|SetTextureParameterValue (Variables|Default|GetDynamicInstanceMaterial) "BrushStroke" (Variables|RenderTextire|GetRender_to_Texture))
  (bind _returnvalue_3 (Rendering|Material|CreateDynamicMaterialInstance "/Game/PaintVR/Materials/MI_PaintBrush.MI_PaintBrush" "None" "None" :!class /Script/Engine.KismetMaterialLibrary))
  (Variables|세팅|SetBrushMaterialInstance _returnvalue_3))

(fn ConstructionScript)

(fn OnPaintVisualTraceLine
  (params (PaintBrush :type BP%20Pen%20Object%20Reference) (HitResult :type Hit%20Result%20Structure))
  (bind _uv (Class|GameplayStatics|FindCollisionUV HitResult))
  (bind (_x _y) (Math|Vector2D|BreakVector2D _uv))
  ;[1 0.5648 0.655] 브러쉬 액터의 정보를 받아 변수로 저장 후 2d Vector 값을 머티리얼 HitPosition 값에 적용
  (Variables|Default|SetBrush PaintBrush)
  (Rendering|Material|SetVectorParameterValue (Variables|세팅|GetBrushMaterialInstance) "HitPosition" (Utilities|Struct|MakeLinearColor _x _y 0.0 1.0) :!class /Script/Engine.MaterialInstanceDynamic)
  ;[1 0.6663 0.5392] 브러쉬 사이즈 머티리얼에 적용
  (Rendering|Material|SetScalarParameterValue (Variables|세팅|GetBrushMaterialInstance) "BrushWidthSize" (Variables|/Game/PaintVR/BluePrints/BP_Pen.BP_Pen_C|GetBrushWidth (Variables|Default|GetBrush)) :!class /Script/Engine.MaterialInstanceDynamic)
  (Rendering|Material|SetScalarParameterValue (Variables|세팅|GetBrushMaterialInstance) "BrushLengthSize" (Variables|/Game/PaintVR/BluePrints/BP_Pen.BP_Pen_C|GetBrushLength (Variables|Default|GetBrush)) :!class /Script/Engine.MaterialInstanceDynamic)
  ;[1 0.9615 0.5347] 브러쉬 컬러 적용
  (Rendering|Material|SetVectorParameterValue (Variables|세팅|GetBrushMaterialInstance) "BrushColor" (Variables|/Game/PaintVR/BluePrints/BP_Pen.BP_Pen_C|GetBrushColor (Variables|Default|GetBrush)) :!class /Script/Engine.MaterialInstanceDynamic)
  ;[0.4637 0.4713 1] 브러쉬 알파값 적용
  (Rendering|Material|SetScalarParameterValue (Variables|세팅|GetBrushMaterialInstance) "BrushStrength" (Variables|/Game/PaintVR/BluePrints/BP_Pen.BP_Pen_C|GetBrushStrength (Variables|Default|GetBrush)) :!class /Script/Engine.MaterialInstanceDynamic)
  ;[0.8058 0.5639 1] 캔버스에 드로우
  (Rendering|DrawMaterialtoRenderTarget (Variables|RenderTextire|GetRender_to_Texture) (Variables|세팅|GetBrushMaterialInstance)))

(fn ExportImage
  ;[0.458 0.4279 1] 경로를 받아 이미지로 저장
  (Class|ImageWriteBlueprintLibrary|ExporttoDisk (Variables|RenderTextire|GetRender_to_Texture) (Utilities|String|Append "/UE_Folder/" "Test.jpg") (Utilities|Struct|MakeImageWriteOptions "JPG" (EventDispatchers|CreateEvent :!event BPCanvasAutoGenFunc) 100)))

(fn BPCanvasAutoGenFunc
  (params (bSuccess :type Boolean))
  (if bSuccess
    (Development|PrintString "Print On")))
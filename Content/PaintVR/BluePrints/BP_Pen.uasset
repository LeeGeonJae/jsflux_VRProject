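; VR paint pen that snaps to the player's right aim controller when grabbed within overlap range and returns to its starting transform on release.
; While the right trigger is held, a looping timer line-traces forward from the pen's arrow and passes hits on BP_Canvas, with itself as brush, to the canvas for painting.
; A dynamic material on the crayon mesh is updated every tick to show the current BrushColor.
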(event EventBeginPlay
  (CallFunction|Init))

(event EventTick
  (params (DeltaSeconds :type Float%20%28single-precision%29))
  (Rendering|Material|SetVectorParameterValue (Variables|디폴트|GetPanMaterialInstance) "Color" (Variables|브러시세팅|GetBrushColor) :!class /Script/Engine.MaterialInstanceDynamic))

(event Input|ActionEvents|InputActionTriggerRight
  (params (Key :type Key%20Structure :default "None"))
  (:Pressed
    (Utilities|Time|SetTimerbyFunctionName 0 "DetectHitCanvasActor" 0.01 true))
  (:Released
    (Utilities|Time|ClearTimerbyFunctionName 0 "DetectHitCanvasActor")))

(event Input|ActionEvents|InputActionGrabRight
  (params (Key :type Key%20Structure :default "None"))
  (:Pressed
    (CallFunction|AttachPen))
  (:Released
    (Transformation|DetachFromActor "KeepRelative" "KeepRelative" "KeepRelative")
    (Transformation|SetWorldTransform (Variables|Default|GetDefaultSceneRoot) (Variables|디폴트|GetPenWorldTransform) false false)))

(fn ConstructionScript)

(fn DetectHitCanvasActor
  (bind _arrowforward (Variables|Default|GetArrowForward))
  (bind _returnvalue (Transformation|GetWorldLocation _arrowforward))
  (bind (_outhit _returnvalue_2) (Class|KismetSystemLibrary|LineTraceSinglebyProfile _returnvalue (+ _returnvalue (* (Math|Vector|GetForwardVector (Transformation|GetWorldRotation _arrowforward)) 1.5e+03)) "BlockAllDynamic" true 0 "None" true))
  (if _returnvalue_2
    (bind _asbp_canvas (Utilities|Casting|CastToBP_Canvas (.HitActor (Collision|BreakHitResult _outhit))))
    (Default|OnPaintVisualTraceLine _asbp_canvas self _outhit)))

(fn Init
  (Utilities|FlowControl|Sequence
    (:then_0
      (bind _returnvalue (Rendering|Material|CreateDynamicMaterialInstance (Variables|Default|GetCrayon) 0 "/Game/PaintVR/Materials/MI_instanceColor.MI_instanceColor" "None" :!class /Script/Engine.PrimitiveComponent))
      (Variables|디폴트|SetPanMaterialInstance _returnvalue))
    (:then_1
      (Input|EnableInput (Game|GetPlayerController 0))
      (bind _returnvalue_2 (Actor|GetActorOfClass "/Game/BluePrint/BP_VRPlayer.BP_VRPlayer_C"))
      (Variables|폰|SetMyVR_Pawn _returnvalue_2))
    (:then_2
      (Variables|디폴트|SetPenWorldTransform (Transformation|GetWorldTransform (Variables|Default|GetDefaultSceneRoot))))))

(fn AttachPen
  (bind _myvr_pawn (Variables|폰|GetMyVR_Pawn))
  (bind _motioncontrollerrightaim (Variables|/Game/BluePrint/BP_VRPlayer.BP_VRPlayer_C|GetMotionControllerRightAim _myvr_pawn))
  (if (Class|PrimitiveComponent|IsOverlappingComponent (Variables|Default|GetSphereCollision) (Variables|/Game/BluePrint/BP_VRPlayer.BP_VRPlayer_C|GetOverlapSphereR (Variables|폰|GetMyVR_Pawn)))
    (Transformation|AttachComponentToComponent _motioncontrollerrightaim "None" "KeepWorld" "KeepWorld" "KeepWorld" true)
    (Transformation|SetActorTransform self (Math|Transform|MakeTransform (Transformation|GetWorldLocation _motioncontrollerrightaim) (Transformation|GetWorldRotation _motioncontrollerrightaim) "1,1,1"))))
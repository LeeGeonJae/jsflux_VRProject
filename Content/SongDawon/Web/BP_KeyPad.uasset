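; BP_KeyPad is a VR actor that presents the UMG_KeyPad widget floating above a motion controller.
; Each tick it moves the widget above the controller and rotates it toward the player camera.
; On BeginPlay it takes the right widget interaction component from BP_VRPlayer and shares it with the keypad UI.
; The right trigger simulates mouse clicks through that component, with actor input toggled by overlaps or enabled via EnableInputActor.
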(event EventOnEndOverlap
  ;[1 1 1] 코멘트
  (Input|DisableInput (Game|GetPlayerController 0)))

(event EventBeginPlay
  ;[1 1 1] 코멘트
  (bind _asbp_vrplayer (Utilities|Casting|CastToBP_VRPlayer (Game|Player|GetPlayerPawn 0)))
  (bind _output_get (Variables|Default|SetWidget%20Interaction%20Right (Variables|/Game/BluePrint/BP_VRPlayer.BP_VRPlayer_C|GetWidgetInteractionRight _asbp_vrplayer)))
  (bind _asumg_key_pad (Utilities|Casting|CastToUMG_KeyPad (UserInterface|GetUserWidgetObject (Variables|Default|GetWidget))))
  (Variables|/Game/SongDawon/Web/UMG_KeyPad.UMG_KeyPad_C|SetWidgetInteraction _asumg_key_pad _output_get))

(event EventTick
  (params (DeltaSeconds :type Float%20%28single-precision%29))
  (bind _widget (Variables|Default|GetWidget))
  ;[1 1 1] 코멘트
  (Transformation|SetWorldLocation (Variables|Default|GetWidget) (+ (Transformation|GetWorldLocation (Variables|Default|GetMotionController)) "0, 0,40.000000") false false)
  (Transformation|SetWorldRotation _widget (Math|Rotator|FindLookatRotation (Transformation|GetWorldLocation _widget) (Transformation|GetActorLocation (Game|GetPlayerCameraManager 0))) false false))

(event EventOnBeginOverlap
  ;[1 1 1] 코멘트
  (Input|EnableInput (Game|GetPlayerController 0)))

(event EventEnableInputActor
  (params (IsEnable :type Boolean))
  ;[1 1 1] 코멘트
  (Input|EnableInput (Game|GetPlayerController 0)))

(event Input|ActionEvents|InputActionTriggerRight
  (params (Key :type Key%20Structure :default "None"))
  (bind _widget_interaction_right (Variables|Default|GetWidget%20Interaction%20Right))
  ;[0.03434 0.03434 0.03434] Menu Input Right
  (:Pressed
    (Class|WidgetInteractionComponent|PressPointerKey _widget_interaction_right "LeftMouseButton"))
  (:Released
    (Class|WidgetInteractionComponent|ReleasePointerKey _widget_interaction_right "LeftMouseButton")))

(fn ConstructionScript)